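; Player controller for the game server that requests the player's character and manages the in-game HUD and settings menu.
; GetCharData on authority calls OC_GetChar, which reads class and gender from the GameInstance profile and passes them through CtS_GetChar to GM_GameServer.CreateChar.
; Escape flip-flops between the lazily created HUD and settings widgets, toggling pause, and SettingsQuit restores the HUD.
; Helper functions forward health and remote-only combat mode to the HUD.
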(event Custom|CtS_GetChar
  (params (Class :type E_Classes%20Enum :default "NewEnumerator0") (Gender :type Boolean))
  (bind _asgm_game_server (Utilities|Casting|CastToGM_GameServer (Game|GetGameMode)))
  (Default|CreateChar _asgm_game_server Class Gender self))

(event Custom|OC_GetChar
  (bind _asgame_instance_mmo (Utilities|Casting|CastToGameInstance_MMO (Game|GetGameInstance)))
  (bind _proifile (Default|GetCurrentProfile _asgame_instance_mmo))
  (CallFunction|CtSGetChar (.class _proifile) (.gender _proifile)))

(event Custom|HUDset
  (Utilities|IsValid (Variables|Default|GetHUD)
    (:Is%20Valid
      (if (not (UserInterface|Viewport|IsinViewport (Variables|Default|GetHUD)))
        (UserInterface|Viewport|AddtoViewport (Variables|Default|GetHUD) 0 :!label _label)))
    (:Is%20Not%20Valid
      (bind _returnvalue (UserInterface|CreateWidget "/Game/UI/HUD_Game.HUD_Game_C"))
      (Variables|Default|SetHUD _returnvalue)
      (goto _label))))

(event Custom|GetCharData
  (Networking|SwitchHasAuthority
    (:Authority
      (CallFunction|OCGetChar))))

(event EventSettingsQuit
  (Widget|RemovefromParent (Variables|Default|GetWB_Settings))
  (CallFunction|HUDset)
  (Game|SetGamePaused false))

(event EventBeginPlay
  (Input|SetInputModeGameandUI self 0 "DoNotLock" true)
  (CallFunction|HUDset))

(event Input|ActionEvents|InputActionEscape
  (params (Key :type Key%20Structure :default "None"))
  (:Pressed
    (Utilities|FlowControl|FlipFlop
      (:A
        (Utilities|IsValid (Variables|Default|GetHUD)
          (:Is%20Valid
            (Widget|RemovefromParent (Variables|Default|GetHUD)))
          (:Is%20Not%20Valid
            _))
        (Utilities|IsValid (Variables|Default|GetWB_Settings)
          (:Is%20Valid
            (if (not (UserInterface|Viewport|IsinViewport (Variables|Default|GetWB_Settings)))
              (UserInterface|Viewport|AddtoViewport (Variables|Default|GetWB_Settings) 0 :!label _label)
              (Game|SetGamePaused true)))
          (:Is%20Not%20Valid
            (bind _returnvalue (UserInterface|CreateWidget "/Game/UI/Settings/WB_Setting.WB_Setting_C"))
            (Variables|Default|SetWB_Settings _returnvalue)
            (goto _label))))
      (:B
        (Widget|RemovefromParent (Variables|Default|GetWB_Settings))
        (CallFunction|HUDset)
        (Game|SetGamePaused false)))))

(fn ConstructionScript)

(fn HUDMode
  (params (bCombat :type Boolean))
  (Networking|SwitchHasAuthority
    (:Remote
      (Default|Mode (Variables|Default|GetHUD) bCombat))))

(fn Health
  (params (InPercent :type Float%20%28single-precision%29))
  (Default|PlayerHealth (Variables|Default|GetHUD) InPercent))