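; Main menu player controller that drives the front-end widget flow: background, main menu, settings (Escape or event) and profile selection.
; Login opens the profiles screen and caches faction and class descriptions from DataTables into arrays.
; SetInfo looks up the selected profile's faction and class via GameInstance_MMO and pushes matching lore text to the profiles widget.
; Enter stores the current profile in the game instance and opens the Test level.
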(event Custom|MainMenu
  (Utilities|IsValid (Variables|Default|GetWB_MainMenu)
    (:Is%20Valid
      _)
    (:Is%20Not%20Valid
      (bind _returnvalue (UserInterface|CreateWidget "/Game/UI/WB_MainMenu.WB_MainMenu_C"))
      (Variables|Default|SetWB_MainMenu _returnvalue)))
  (UserInterface|Viewport|AddtoViewport (Variables|Default|GetWB_MainMenu) 0))

(event Custom|Login
  (Widget|RemovefromParent (Variables|Default|GetWB_MainMenu))
  (bind _returnvalue (UserInterface|CreateWidget "/Game/UI/WB_Profiles.WB_Profiles_C"))
  (bind _output_get (Variables|Default|SetWB_Profiles _returnvalue))
  (UserInterface|Viewport|AddtoViewport _output_get 0)
  (bind _outrownames (DataTable|GetDataTableRowNames "/Game/Data/DT_Factions.DT_Factions"))
  (for _array_element _outrownames
    (bind _returnvalue_2 (Utilities|GetDataTableRow "/Game/Data/DT_Factions.DT_Factions" _array_element)
      (:then
        (Utilities|Array|Add (Variables|Default|GetFactionsInfo) (Utilities|Struct|MakeF_CFInfo (Utilities|String|EnumtoString (.factionname _returnvalue_2)) (.story _returnvalue_2))))))
  (bind _outrownames_2 (DataTable|GetDataTableRowNames "/Game/Data/DT_Classes.DT_Classes"))
  (for _array_element_2 _outrownames_2
    (bind _returnvalue_3 (Utilities|GetDataTableRow "/Game/Data/DT_Classes.DT_Classes" _array_element_2)
      (:then
        (Utilities|Array|Add (Variables|Default|GetClassInfo) (Utilities|Struct|MakeF_CFInfo (Utilities|String|EnumtoString (.classname _returnvalue_3)) (.classdescription _returnvalue_3)))))))

(event Custom|Enter
  (bind _asgame_instance_mmo (Utilities|Casting|CastToGameInstance_MMO (Game|GetGameInstance)))
  (Default|SetCurrentProfile _asgame_instance_mmo (Variables|Default|GetProfileName))
  (Game|OpenLevel(byName) "Test"))

(event EventBeginPlay
  (bind _returnvalue (UserInterface|CreateWidget "/Game/UI/WB_Background.WB_Background_C"))
  (UserInterface|Viewport|AddtoViewport _returnvalue 0)
  (Input|SetInputModeUIOnly self 0 "DoNotLock")
  (CallFunction|MainMenu))

(event EventSettingsQuit
  (CallFunction|MainMenu))

(event EventSettingsShow
  (Widget|RemovefromParent (Variables|Default|GetWB_MainMenu))
  (bind _returnvalue (UserInterface|CreateWidget "/Game/UI/Settings/WB_Setting.WB_Setting_C"))
  (UserInterface|Viewport|AddtoViewport _returnvalue 0))

(event Input|ActionEvents|InputActionEscape
  (params (Key :type Key%20Structure :default "None"))
  (:Pressed
    (Widget|RemovefromParent (Variables|Default|GetWB_MainMenu))
    (bind _returnvalue (UserInterface|CreateWidget "/Game/UI/Settings/WB_Setting.WB_Setting_C"))
    (UserInterface|Viewport|AddtoViewport _returnvalue 0)))

(fn ConstructionScript)

(fn SetInfo
  (params (ProfileName :type String))
  (bind _output_get (Variables|Default|SetProfileName ProfileName))
  (bind _asgame_instance_mmo (Utilities|Casting|CastToGameInstance_MMO (Game|GetGameInstance)))
  (bind (_array_element_faction _array_element_class) (Default|GetFactionClass _asgame_instance_mmo _output_get))
  (bind _array_element (Utilities|Array|ForEachLoopwithBreak (Variables|Default|GetFactionsInfo) :!label _label)
    (:LoopBody
      (if (Utilities|Enum|Equal(Enum) (Utilities|String|EnumtoString _array_element_faction) (.name _array_element))
        (LocalVariables|SetFactionStory (.story _array_element))
        (goto _label Break)))
    (:Completed
      (bind _array_element_2 (Utilities|Array|ForEachLoopwithBreak (Variables|Default|GetClassInfo) :!label _label_2)
        (:LoopBody
          (if (Utilities|Enum|Equal(Enum) (Utilities|String|EnumtoString _array_element_class) (.name _array_element_2))
            (LocalVariables|SetClassStory (.story _array_element_2))
            (goto _label_2 Break)))
        (:Completed
          (Default|SetFaction&Class (Variables|Default|GetWB_Profiles) (Utilities|Text|ToText(String) (Utilities|String|EnumtoString _array_element_faction)) (LocalVariables|GetFactionStory) (Utilities|Text|ToText(String) (Utilities|String|EnumtoString _array_element_class)) (LocalVariables|GetClassStory)))))))