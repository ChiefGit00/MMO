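; Ctrl_Game is the gameplay controller that requests creation of the player's character from the selected profile.
; On BeginPlay it sets game-only input and calls OC_GetChar, which reads the current profile's class and gender from GameInstance_MMO.
; It passes them to CtS_GetChar, which has GM_Game create the character for this controller.
; The event prefixes suggest an owning-client to server hand-off.
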(event Custom|CtS_GetChar
  (params (Class :type E_Classes%20Enum :default "NewEnumerator0") (Gender :type Boolean))
  (bind _asgm_game (Utilities|Casting|CastToGM_Game (Game|GetGameMode)))
  (Default|CreateChar _asgm_game Class Gender self))

(event Custom|OC_GetChar
  (bind _asgame_instance_mmo (Utilities|Casting|CastToGameInstance_MMO (Game|GetGameInstance)))
  (bind _proifile (Default|GetCurrentProfile _asgame_instance_mmo))
  (CallFunction|CtSGetChar (.class _proifile) (.gender _proifile)))

(event EventBeginPlay
  (Input|SetInputModeGameOnly self)
  (CallFunction|OCGetChar))

(fn ConstructionScript)