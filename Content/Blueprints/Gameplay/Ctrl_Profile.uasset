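; Player controller for the character profile creation screen, which shows a profile HUD and spawns a showcase character.
; Switcher functions cycle with wraparound through faction and class data table rows, updating the HUD and setting the showcase mesh by class and gender.
; CreateProfile passes the name, faction, class and gender to the MMO GameInstance, then opens the Test level.
; Escape swaps the HUD for a settings widget, and SettingsQuit restores it.
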(event Custom|SetHUD
  (Utilities|IsValid (Variables|Default|GetHUD)
    (:Is%20Valid
      _)
    (:Is%20Not%20Valid
      (bind _returnvalue (UserInterface|CreateWidget "/Game/UI/WB_HUD_Profiles.WB_HUD_Profiles_C"))
      (Variables|Default|SetHUD _returnvalue)))
  (UserInterface|Viewport|AddtoViewport (Variables|Default|GetHUD) 0))

(event EventBeginPlay
  (CallFunction|SetHUD)
  (Input|SetInputModeGameandUI self 0 "DoNotLock" true)
  (|InitDataTables)
  (bind _returnvalue (Game|SpawnActorfromClass "/Game/Blueprints/Actors/Characters/BP_Char_Showcase.BP_Char_Showcase_C" (Math|Transform|MakeTransform "0, 0, 0" "0,-100.000000, 0" "1,1,1") "Undefined" 0 0))
  (Variables|Default|SetSpawnedChar _returnvalue)
  (CallFunction|ClassSwitcher)
  (CallFunction|FactionSwitcher))

(event EventSettingsQuit
  (CallFunction|SetHUD))

(event Input|ActionEvents|InputActionEscape
  (params (Key :type Key%20Structure :default "None"))
  (:Pressed
    (Development|PrintString "Hello")
    (Widget|RemovefromParent (Variables|Default|GetHUD))
    (bind _returnvalue (UserInterface|CreateWidget "/Game/UI/WB_Setting.WB_Setting_C"))
    (UserInterface|Viewport|AddtoViewport _returnvalue 0)))

(fn ConstructionScript)

(fn FactionSwitcher
  (params (IndexDelta :type Integer))
  (bind _output_get (Variables|Default|SetcurrentFactionsRow (+ IndexDelta (Variables|Default|GetcurrentFactionsRow))))
  (if (< _output_get 0)
    (Variables|Default|SetcurrentFactionsRow (- (Variables|Default|GetFactionsDTLength) 1))
    (elif (== _output_get (Variables|Default|GetFactionsDTLength))
      (Variables|Default|SetcurrentFactionsRow 0)))
  (bind _returnvalue (Utilities|GetDataTableRow "/Game/Data/DT_Factions.DT_Factions" (Utilities|Array|Get(acopy) (Variables|Default|GetFactionsDTRows) (Variables|Default|GetcurrentFactionsRow)))
    (:then
      (Default|SetFaction (Variables|Default|GetHUD) (Utilities|Text|ToText(String) (Utilities|String|EnumtoString (.factionname _returnvalue))) (.story _returnvalue) (.symbol _returnvalue)))))

(fn ClassSwitcher
  (params (IndexDelta :type Integer))
  (bind _output_get (Variables|Default|SetcurrentClassRow (+ IndexDelta (Variables|Default|GetcurrentClassRow))))
  (if (< _output_get 0)
    (Variables|Default|SetcurrentClassRow (- (Variables|Default|GetClassesDTLength) 1))
    (elif (== _output_get (Variables|Default|GetClassesDTLength))
      (Variables|Default|SetcurrentClassRow 0)))
  (bind _returnvalue (Utilities|GetDataTableRow "/Game/Data/DT_Classes.DT_Classes" (Utilities|Array|Get(acopy) (Variables|Default|GetClassesDTRows) (Variables|Default|GetcurrentClassRow)))
    (:then
      (Default|SetClass (Variables|Default|GetHUD) (Utilities|Text|ToText(String) (Utilities|String|EnumtoString (.classname _returnvalue))) (.classdescription _returnvalue) (.classicon _returnvalue))
      (Default|SetMesh (Variables|Default|GetSpawnedChar) (select (Variables|Default|GetbGender) (.sk_mesh_m _returnvalue) (.sk_mesh_f _returnvalue))))))

(fn CreateProfile
  (params (ProfileName :type String))
  (bind _returnvalue (Utilities|GetDataTableRow "/Game/Data/DT_Classes.DT_Classes" (Utilities|Array|Get(acopy) (Variables|Default|GetClassesDTRows) (Variables|Default|GetcurrentClassRow)))
    (:then
      (bind _returnvalue_2 (Utilities|GetDataTableRow "/Game/Data/DT_Factions.DT_Factions" (Utilities|Array|Get(acopy) (Variables|Default|GetFactionsDTRows) (Variables|Default|GetcurrentFactionsRow)))
        (:then
          (bind _asgame_instance_mmo (Utilities|Casting|CastToGameInstance_MMO (Game|GetGameInstance)))
          (Default|CreateProfile _asgame_instance_mmo ProfileName (.factionname _returnvalue_2) (.classname _returnvalue) (Variables|Default|GetbGender))
          (Game|OpenLevel(byName) "Test"))))))