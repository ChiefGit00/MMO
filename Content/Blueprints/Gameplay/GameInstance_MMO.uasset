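; MMO game instance that persists the server IP and the player's character profiles through a SaveGame_MMO object in the "SaveGame" slot.
; InitSaveGame lazily loads or creates that object and caches it, though SetCurrentProfile and GetFactionClass skip this step.
; Profile functions create, select, delete and query entries by name or by a stored current index, and every change is saved to the slot immediately.
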(fn InitSaveGame
  (Utilities|IsValid (Variables|Default|GetObjSaveGame)
    (:Is%20Not%20Valid
      (bind _returnvalue (SaveGame|DoesSaveGameExist "SaveGame"))
      (if _returnvalue
        (bind _returnvalue_2 (SaveGame|LoadGamefromSlot "SaveGame"))
        (bind _assave_game_mmo (Utilities|Casting|CastToSaveGame_MMO _returnvalue_2))
        (Variables|Default|SetObjSaveGame _assave_game_mmo)
        (else
          (bind _returnvalue_3 (SaveGame|CreateSaveGameObject "/Game/Blueprints/Gameplay/SaveGame_MMO.SaveGame_MMO_C"))
          (Variables|Default|SetObjSaveGame _returnvalue_3))))))

(fn GetServerIP
  (CallFunction|InitSaveGame)
  (return (Variables|/Game/Blueprints/Gameplay/SaveGame_MMO.SaveGame_MMO_C|GetServerIP (Variables|Default|GetObjSaveGame))))

(fn SaveServerIP
  (params (ServerIP :type String))
  (bind _objsavegame (Variables|Default|GetObjSaveGame))
  (CallFunction|InitSaveGame)
  (Variables|/Game/Blueprints/Gameplay/SaveGame_MMO.SaveGame_MMO_C|SetServerIP _objsavegame ServerIP)
  (SaveGame|SaveGametoSlot _objsavegame "SaveGame"))

(fn CreateProfile
  (params (ProfileName :type String) (Faction :type E_Factions%20Enum :default "NewEnumerator0") (ClassName :type E_Classes%20Enum :default "NewEnumerator0") (Gender :type Boolean))
  (bind _objsavegame (Variables|Default|GetObjSaveGame))
  (CallFunction|InitSaveGame)
  (bind _returnvalue (Utilities|Array|Add (Variables|/Game/Blueprints/Gameplay/SaveGame_MMO.SaveGame_MMO_C|GetCharProfiles (Variables|Default|GetObjSaveGame)) (Utilities|Struct|MakeF_PlayerCharData ProfileName Faction ClassName Gender 0 0 0 0 (Class|KismetMathLibrary|GetDate (Math|DateTime|Now)) "+00000000.00:00:00.000000000")))
  (Variables|/Game/Blueprints/Gameplay/SaveGame_MMO.SaveGame_MMO_C|SetCurrentProfileIndex _objsavegame _returnvalue)
  (SaveGame|SaveGametoSlot _objsavegame "SaveGame"))

(fn GetCurrentProfile
  (bind _objsavegame (Variables|Default|GetObjSaveGame))
  (CallFunction|InitSaveGame)
  (return (Utilities|Array|Get(acopy) (Variables|/Game/Blueprints/Gameplay/SaveGame_MMO.SaveGame_MMO_C|GetCharProfiles _objsavegame) (Variables|/Game/Blueprints/Gameplay/SaveGame_MMO.SaveGame_MMO_C|GetCurrentProfileIndex _objsavegame))))

(fn GetAllProfiles
  (CallFunction|InitSaveGame)
  (return (Variables|/Game/Blueprints/Gameplay/SaveGame_MMO.SaveGame_MMO_C|GetCharProfiles (Variables|Default|GetObjSaveGame))))

(fn SetCurrentProfile
  (params (ProfileName :type String))
  (bind _index (CallFunction|FindProfileIndex ProfileName))
  (Variables|/Game/Blueprints/Gameplay/SaveGame_MMO.SaveGame_MMO_C|SetCurrentProfileIndex (Variables|Default|GetObjSaveGame) _index)
  (SaveGame|SaveGametoSlot (Variables|Default|GetObjSaveGame) "SaveGame"))

(fn DeleteProfile
  (params (PeifileName :type String))
  (CallFunction|InitSaveGame)
  (bind _index (CallFunction|FindProfileIndex PeifileName))
  (Utilities|Array|RemoveIndex (Variables|/Game/Blueprints/Gameplay/SaveGame_MMO.SaveGame_MMO_C|GetCharProfiles (Variables|Default|GetObjSaveGame)) _index)
  (SaveGame|SaveGametoSlot (Variables|Default|GetObjSaveGame) "SaveGame"))

(fn FindProfileIndex
  (params (ProfileName :type String))
  (bind (_array_element _array_index) (Utilities|Array|ForEachLoopwithBreak (Variables|/Game/Blueprints/Gameplay/SaveGame_MMO.SaveGame_MMO_C|GetCharProfiles (Variables|Default|GetObjSaveGame)))
    (:LoopBody
      (if (Utilities|Enum|Equal(Enum) (.profilename _array_element) ProfileName)
        (return _array_index)))))

(fn GetFactionClass
  (params (ProfileName :type String))
  (bind _array_element (Utilities|Array|ForEachLoopwithBreak (Variables|/Game/Blueprints/Gameplay/SaveGame_MMO.SaveGame_MMO_C|GetCharProfiles (Variables|Default|GetObjSaveGame)))
    (:LoopBody
      (if (Utilities|Enum|Equal(Enum) ProfileName (.profilename _array_element))
        (LocalVariables|SetFaction (.faction _array_element))
        (LocalVariables|SetClass (.class _array_element))))
    (:Completed
      (return (LocalVariables|GetFaction) (LocalVariables|GetClass)))))