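; Playable character with gendered mesh selection, controller-yaw-relative movement, mouse look, melee attacks and dodge rolls.
; Equipping attaches a weapon to the right-hand socket and notifies the anim instance; dropping detaches and clears it.
; With a weapon, each mouse button alternates two attack montage sections via FlipFlop, setting the weapon's Attack flag until completion.
; Holding Jump opens Gates that let W/A/S/D presses play directional roll montages.
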(event Custom|SetMesh
  (params (Gender :type Boolean))
  (Class|SkinnedMeshComponent|SetSkeletalMesh (Variables|Character|GetMesh) (select Gender (Variables|Default|GetMaleMesh) (Variables|Default|GetFemaleMesh)) true))

(event Custom|EquipWeapon
  (params (Weapon :type WB%20Weapon%20Object%20Reference))
  (Utilities|IsValid (Variables|Default|GetWeapon)
    (:Is%20Valid
      (CallFunction|DropEquip))
    (:Is%20Not%20Valid
      _))
  (bind _output_get (Variables|Default|SetWeapon Weapon))
  (Transformation|AttachComponentToComponent _output_get (Variables|Character|GetMesh) "hand_rSocket" "SnapToTarget" "SnapToTarget" "SnapToTarget" true)
  (bind _output_get_2 (Variables|Default|SetbWeapon true))
  (Class|BPIAnimationGame|EquipedWeapon(Message) (Components|SkeletalMesh|GetAnimInstance (Variables|Character|GetMesh)) _output_get_2))

(event Custom|DropEquip
  (Utilities|IsValid (Variables|Default|GetWeapon)
    (:Is%20Valid
      (Default|Drop (Variables|Default|GetWeapon))
      (Transformation|DetachFromComponent (Variables|/Game/Blueprints/Actors/Weapons/WB_Weapon.WB_Weapon_C|GetSkeletalMesh (Variables|Default|GetWeapon)) "KeepWorld" "KeepWorld" "KeepWorld" true)
      (bind _output_get (Variables|Default|SetbWeapon false))
      (Default|CallWeaponEquiped _output_get)
      (Variables|Default|SetWeapon 0)
      (Class|BPIAnimationGame|EquipedWeapon(Message) (Components|SkeletalMesh|GetAnimInstance (Variables|Character|GetMesh)) false))))

(event Input|ActionEvents|InputActionDropEquip
  (params (Key :type Key%20Structure :default "None"))
  (:Pressed
    (Utilities|IsValid (Variables|Default|GetWeapon)
      (:Is%20Valid
        (Default|Drop (Variables|Default|GetWeapon))
        (Transformation|DetachFromComponent (Variables|/Game/Blueprints/Actors/Weapons/WB_Weapon.WB_Weapon_C|GetSkeletalMesh (Variables|Default|GetWeapon)) "KeepWorld" "KeepWorld" "KeepWorld" true)
        (bind _output_get (Variables|Default|SetbWeapon false))
        (Default|CallWeaponEquiped _output_get)
        (Variables|Default|SetWeapon 0)
        (Class|BPIAnimationGame|EquipedWeapon(Message) (Components|SkeletalMesh|GetAnimInstance (Variables|Character|GetMesh)) false)))))

(event Input|ActionEvents|InputActionMouseLeft
  (params (Key :type Key%20Structure :default "None"))
  (bind _mesh (Variables|Character|GetMesh))
  (:Pressed
    (if (Variables|Default|GetbWeapon)
      (Variables|/Game/Blueprints/Actors/Weapons/WB_Weapon.WB_Weapon_C|SetbAttack (Variables|Default|GetWeapon) true)
      (Utilities|FlowControl|FlipFlop
        (:A
          (Animation|Montage|PlayMontage _mesh "/Game/SkeletalMeshes/ProtoCharacters/ABP/AM_Attack.AM_Attack" 1.0 0.0 "Attack01"
            (:OnCompleted
              _)))
        (:B
          (Animation|Montage|PlayMontage _mesh "/Game/SkeletalMeshes/ProtoCharacters/ABP/AM_Attack.AM_Attack" 1.0 0.0 "Attack03"
            (:OnCompleted
              _))))
      (Variables|/Game/Blueprints/Actors/Weapons/WB_Weapon.WB_Weapon_C|SetbAttack (Variables|Default|GetWeapon) false))))

(event Input|ActionEvents|InputActionMouseRight
  (params (Key :type Key%20Structure :default "None"))
  (bind _mesh (Variables|Character|GetMesh))
  (:Pressed
    (if (Variables|Default|GetbWeapon)
      (Variables|/Game/Blueprints/Actors/Weapons/WB_Weapon.WB_Weapon_C|SetbAttack (Variables|Default|GetWeapon) true)
      (Utilities|FlowControl|FlipFlop
        (:A
          (Animation|Montage|PlayMontage _mesh "/Game/SkeletalMeshes/ProtoCharacters/ABP/AM_Attack.AM_Attack" 1.0 0.0 "Attack02"
            (:OnCompleted
              _)))
        (:B
          (Animation|Montage|PlayMontage _mesh "/Game/SkeletalMeshes/ProtoCharacters/ABP/AM_Attack.AM_Attack" 1.0 0.0 "Attack04"
            (:OnCompleted
              _))))
      (Variables|/Game/Blueprints/Actors/Weapons/WB_Weapon.WB_Weapon_C|SetbAttack (Variables|Default|GetWeapon) false))))

(event Input|ActionEvents|InputActionJump
  (params (Key :type Key%20Structure :default "None"))
  (:Pressed
    (Utilities|FlowControl|Sequence
      (:then_0
        (Utilities|FlowControl|Gate true) ; enters at Open
      )
      (:then_1
        (Utilities|FlowControl|Gate true) ; enters at Open
      )
      (:then_2
        (Utilities|FlowControl|Gate true) ; enters at Open
      )
      (:then_3
        (Utilities|FlowControl|Gate true) ; enters at Open
      )))
  (:Released
    (Utilities|FlowControl|Sequence
      (:then_0
        (Utilities|FlowControl|Gate true) ; enters at Close
      )
      (:then_1
        (Utilities|FlowControl|Gate true) ; enters at Close
      )
      (:then_2
        (Utilities|FlowControl|Gate true) ; enters at Close
      )
      (:then_3
        (Utilities|FlowControl|Gate true) ; enters at Close
      ))))

(event Input|AxisEvents|InputAxisAxisX
  (params (AxisValue :type Float%20%28single-precision%29))
  (Pawn|Input|AddControllerYawInput AxisValue))

(event Input|AxisEvents|InputAxisAxixY
  (params (AxisValue :type Float%20%28single-precision%29))
  (Pawn|Input|AddControllerPitchInput AxisValue))

(event Input|AxisEvents|InputAxisMoveForward
  (params (AxisValue :type Float%20%28single-precision%29))
  (Pawn|Input|AddMovementInput (Math|Vector|GetForwardVector (Math|Rotator|MakeRotator 0.0 0.0 (.yaw (Pawn|GetControlRotation :!class /Script/Engine.Pawn)))) AxisValue false))

(event Input|AxisEvents|InputAxisMoveRight
  (params (AxisValue :type Float%20%28single-precision%29))
  (Pawn|Input|AddMovementInput (Math|Vector|GetRightVector (Math|Rotator|MakeRotator 0.0 0.0 (.yaw (Pawn|GetControlRotation :!class /Script/Engine.Pawn)))) AxisValue false))

(event Input|KeyboardEvents|W
  (params (Key :type Key%20Structure :default "None"))
  (:Pressed
    (Utilities|FlowControl|Gate true :!label _label
      (:Exit
        (Animation|Montage|PlayMontage (Variables|Character|GetMesh) "/Game/SkeletalMeshes/ProtoCharacters/ABP/AM_Rolls.AM_Rolls" 1.0 0.0 "RollForward"
          (:OnCompleted
            (goto _label Close)))))))

(event Input|KeyboardEvents|S
  (params (Key :type Key%20Structure :default "None"))
  (:Pressed
    (Utilities|FlowControl|Gate true :!label _label
      (:Exit
        (Animation|Montage|PlayMontage (Variables|Character|GetMesh) "/Game/SkeletalMeshes/ProtoCharacters/ABP/AM_Rolls.AM_Rolls" 1.0 0.0 "RollBack"
          (:OnCompleted
            (goto _label Close)))))))

(event Input|KeyboardEvents|A
  (params (Key :type Key%20Structure :default "None"))
  (:Pressed
    (Utilities|FlowControl|Gate true :!label _label
      (:Exit
        (Animation|Montage|PlayMontage (Variables|Character|GetMesh) "/Game/SkeletalMeshes/ProtoCharacters/ABP/AM_Rolls.AM_Rolls" 1.0 0.0 "RollLeft"
          (:OnCompleted
            (goto _label Close)))))))

(event Input|KeyboardEvents|D
  (params (Key :type Key%20Structure :default "None"))
  (:Pressed
    (Utilities|FlowControl|Gate true :!label _label
      (:Exit
        (Animation|Montage|PlayMontage (Variables|Character|GetMesh) "/Game/SkeletalMeshes/ProtoCharacters/ABP/AM_Rolls.AM_Rolls" 1.0 0.0 "RollRight"
          (:OnCompleted
            (goto _label Close)))))))

(fn ConstructionScript)