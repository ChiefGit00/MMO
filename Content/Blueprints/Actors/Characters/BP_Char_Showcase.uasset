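; BP_Char_Showcase is a display character that shows a swappable skeletal mesh slowly rotating on yaw.
; Tick adds a small per-frame rotation through a gate, which opens after a short delay following BeginPlay.
; SetMesh swaps the mesh and calls Reset, which zeroes the rotation, closes the gate and reruns the delayed opening.
; SetClassColour is an empty event.
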(event Custom|Reset
  (Utilities|FlowControl|Sequence
    (:then_0
      (Transformation|SetRelativeRotation (Variables|Default|GetSkeletalMesh) "0, 0, 0" false false)
      (Utilities|FlowControl|Gate true) ; enters at Close
    )
    (:then_1
      (Utilities|FlowControl|Delay 1.0)
      (Utilities|FlowControl|Gate true) ; enters at Open
    )))

(event Custom|SetClassColour)

(event EventTick
  (params (DeltaSeconds :type Float%20%28single-precision%29))
  (Utilities|FlowControl|Gate true
    (:Exit
      (Transformation|AddLocalRotation (Variables|Default|GetSkeletalMesh) "0,0.200000, 0" false false))))

(event EventBeginPlay
  (Utilities|FlowControl|Delay 1.0)
  (Utilities|FlowControl|Gate true) ; enters at Open
)

(fn ConstructionScript)

(fn SetMesh
  (params (Mesh :type Skeletal%20Mesh%20Object%20Reference))
  (Class|SkinnedMeshComponent|SetSkeletalMesh (Variables|Default|GetSkeletalMesh) Mesh true)
  (CallFunction|Reset))