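; BP_CharGame is a playable MMO character with control-yaw-relative movement and mouse-look style axis input.
; On BeginPlay it fetches the current profile from GameInstance_MMO, then calls SetSkeletalMesh with no mesh specified.
; A Select on the profile's class name (Human, Beast, Element, Undead, Demon) is left unused, so class-based appearance is not wired.
; Move axes follow controller yaw only, while look axes feed controller yaw and pitch.
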(event EventBeginPlay
  (bind _asgame_instance_mmo (Utilities|Casting|CastToGameInstance_MMO (Game|GetGameInstance)))
  (bind _proifile (Default|GetCurrentProfile _asgame_instance_mmo))
  (Class|SkinnedMeshComponent|SetSkeletalMesh (Variables|Character|GetMesh) 0 true))

(event Input|AxisEvents|InputAxisAxisX
  (params (AxisValue :type Float%20%28single-precision%29))
  (Pawn|Input|AddControllerYawInput AxisValue))

(event Input|AxisEvents|InputAxisAxixY
  (params (AxisValue :type Float%20%28single-precision%29))
  (Pawn|Input|AddControllerPitchInput AxisValue))

(event Input|AxisEvents|InputAxisMoveForward
  (params (AxisValue :type Float%20%28single-precision%29))
  (Pawn|Input|AddMovementInput (Math|Vector|GetForwardVector (Math|Rotator|MakeRotator 0.0 0.0 (.yaw (Pawn|GetControlRotation :!class /Script/Engine.Pawn)))) AxisValue false))

(event Input|AxisEvents|InputAxisMoveRight
  (params (AxisValue :type Float%20%28single-precision%29))
  (Pawn|Input|AddMovementInput (Math|Vector|GetRightVector (Math|Rotator|MakeRotator 0.0 0.0 (.yaw (Pawn|GetControlRotation :!class /Script/Engine.Pawn)))) AxisValue false))

(fn ConstructionScript)